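; Animation modifier that auto-places SKG footstep sound notifies along an animation sequence.
; On apply, it clears existing notifies, then adds one every SpaceApart from StartTime up to TotalLength, alternating left and right foot bones from a configurable first foot.
; Each notify gets its foot bone, trace channel and physical material effect tag; revert removes the notifies by name.
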(event `SetInitialValues`
  (set `self.Time` (`self.StartTime`))
  (if (`self.FirstFootIsRight`)
    (set `self.SelectedBone` (`self.RightFootName`))
    (else
      (set `self.SelectedBone` (`self.LeftFootName`))))
  (set `self.StepCount` (/ (`self.TotalLength`) (`self.SpaceApart`))))

(event `RemoveFootstepNotifies`
  (params (Sequence :type "AnimSequence Object Reference"))
  (`AnimationBlueprintLibrary.RemoveAnimationNotifyEventsByName` Sequence "USKGPlayFootstepSound"))

(event `self.OnApply`
  (params (AnimationSequence :type "AnimSequence Object Reference"))
  (`self.RemoveFootstepNotifies` AnimationSequence)
  (`self.SetInitialValues`)
  (for _ (range (+ (`self.StepCount`) 1))
    (`self.AddNotify` AnimationSequence (`self.Time`) (`self.SelectedBone`))
    (set `self.Time` (+ (`self.Time`) (`self.SpaceApart`)))
    (`self.FlipSelectedBone`)
    (if (> (`self.Time`) (`self.TotalLength`))
      (break))))

(event `self.OnRevert`
  (params (AnimationSequence :type "AnimSequence Object Reference"))
  (`self.RemoveFootstepNotifies` AnimationSequence))

(fn `AddNotify`
  (params (Sequence :type "AnimSequence Object Reference") (Position :type "Float (double-precision)") (Bone :type Name))
  (locals (Notify :type "UAnimNotify_SKGPlayFootstepSound Object Reference"))
  (bind _returnvalue (`AnimationBlueprintLibrary.AddAnimationNotifyEvent` Sequence "1" Position "/Script/SKGPhysicalMaterialModule.UAnimNotify_SKGPlayFootstepSound"))
  (bind _asuanim_notify_skgplay_footstep_sound (cast `UAnimNotify_SKGPlayFootstepSound` _returnvalue))
  (set `local.Notify` _asuanim_notify_skgplay_footstep_sound)
  (`UAnimNotify_SKGPlayFootstepSound.SetFootBoneName` (`local.Notify`) (`local.Bone`))
  (`UAnimNotify_SKGPlayFootstepSound.SetTraceChannel` (`local.Notify`) (`self.CollisionChannel`))
  (`UAnimNotify_SKGPlayFootstepSound.SetPhysicalMaterialEffectTag` (`local.Notify`) (`self.PhysicalMaterialTag`)))

(fn `FlipSelectedBone`
  (if (== (`self.SelectedBone`) (`self.LeftFootName`))
    (set `self.SelectedBone` (`self.RightFootName`))
    (else
      (set `self.SelectedBone` (`self.LeftFootName`)))))