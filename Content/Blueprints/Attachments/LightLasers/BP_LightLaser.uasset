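; Weapon light/laser attachment that keeps its visible light beam, light blinder and laser blinder in sync with its SKGLightLaser component.
; Component events show or hide these visuals on mode changes and strobe pulses, suppressing them while infrared is active.
; Leaving infrared restores the laser blinder if the laser is on, and the light visuals only if both are on.
; Interact calls are forwarded to the parent that has the firearm component.
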(event `self.SKGLightLaser.OnLightModeChanged`
  (params (LightMode :type "ESKGLightMode Enum" :default "Off"))
  (bind _lightblinder (`self.LightBlinder`))
  (bind _lightbeam (`self.LightBeam`))
  (switch `ESKGLightMode` LightMode
    (:`Off`
      (`SceneComponent.SetHiddenInGame` _lightbeam true false)
      (`SceneComponent.SetHiddenInGame` _lightblinder true false))
    (:`On`
      (if (not (`SKGLightLaserComponent.bDeviceInfraredOn` (`self.SKGLightLaser`))) :!label _label
        (`SceneComponent.SetHiddenInGame` _lightbeam false false)
        (`SceneComponent.SetHiddenInGame` _lightblinder false false)))
    (:`Strobe`
      (goto _label))))

(event `self.SKGLightLaser.OnLightStrobed`
  (params (bOn :type Boolean))
  (bind _lightblinder (`self.LightBlinder`))
  (bind _lightbeam (`self.LightBeam`))
  (if (`SKGLightLaserComponent.bDeviceInfraredOn` (`self.SKGLightLaser`))
    _
    (elif bOn
      (`SceneComponent.SetHiddenInGame` _lightbeam false false)
      (`SceneComponent.SetHiddenInGame` _lightblinder false false)
      (else
        (`SceneComponent.SetHiddenInGame` _lightbeam true false)
        (`SceneComponent.SetHiddenInGame` _lightblinder true false)))))

(event `self.SKGLightLaser.OnLaserStateChanged`
  (params (LaserMode :type "ESKGLaserMode Enum" :default "Off"))
  (bind _laserblinder (`self.LaserBlinder`))
  (switch `ESKGLaserMode` LaserMode
    (:`Off`
      (`SceneComponent.SetHiddenInGame` _laserblinder true false))
    (:`On`
      (if (not (`SKGLightLaserComponent.bDeviceInfraredOn` (`self.SKGLightLaser`)))
        (`SceneComponent.SetHiddenInGame` _laserblinder false false)))))

(event `self.SKGLightLaser.OnInfraredModeChanged`
  (params (bInInfraredMode :type Boolean))
  (bind _lightbeam (`self.LightBeam`))
  (bind _lightblinder (`self.LightBlinder`))
  (bind _laserblinder (`self.LaserBlinder`))
  (if bInInfraredMode
    (`SceneComponent.SetHiddenInGame` _laserblinder true false)
    (`SceneComponent.SetHiddenInGame` _lightbeam true false)
    (`SceneComponent.SetHiddenInGame` _lightblinder true false)
    (elif (`SKGLightLaserComponent.IsLaserOn` (`self.SKGLightLaser`))
      (`SceneComponent.SetHiddenInGame` _laserblinder false false)
      (if (`SKGLightLaserComponent.IsLightOn` (`self.SKGLightLaser`))
        (`SceneComponent.SetHiddenInGame` _lightbeam false false)
        (`SceneComponent.SetHiddenInGame` _lightblinder false false)))))

(event `self.Interact`
  (params (Pawn :type "Pawn Object Reference"))
  (bind _returnvalue (`SKGShooterFrameworkHelpers.GetParentWithFirearmComponent` self))
  (`/Engine/EditorBlueprintResources/StandardMacros.IsValid` _returnvalue
    (:`Is Valid`
      (bind _asinteract_interface (cast `InteractInterface` _returnvalue))
      (`InteractInterface.Interact` _asinteract_interface null))))

(fn `UserConstructionScript`)