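; Flip-to-side magnifier attachment that pairs with a firearm optic and switches aiming between itself and that optic.
; LinkOptic sphere-traces sideways to pick the nearest optic, which receives forwarded reticle cycle, brightness and night vision changes.
; Flips are cooldown-limited, set locally, sent to the server and applied through HandleFlippedResult on BeginPlay, linking and OnRep, driving animations and the firearm's aiming device.
; Destruction returns aim to the linked optic for the local player.
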(event `self.ReceiveBeginPlay`
  (`self.HandleFlippedResult`))

(event `SetAimToMagnifier`
  (bind _skgproceduralanim_magnifier (`self.SKGProceduralAnim_Magnifier`))
  (bind _linkedoptic (`self.LinkedOptic`))
  (`/Engine/EditorBlueprintResources/StandardMacros.IsValid` _linkedoptic
    (:`Is Valid`
      (`SKGProceduralAnimComponent.SetCanAim` (`SKGShooterFrameworkHelpers.GetProceduralAnimComponent` _linkedoptic) false)
      (`SKGProceduralAnimComponent.SetCanAim` _skgproceduralanim_magnifier true)
      (`SKGFirearmComponent.SetAimingDevice` (`SKGShooterFrameworkHelpers.GetParentFirearmComponent` self) _skgproceduralanim_magnifier (`self.GetIsAiming`)))))

(event `SetAimToLinkedOptic`
  (bind _linkedoptic (`self.LinkedOptic`))
  (`/Engine/EditorBlueprintResources/StandardMacros.IsValid` _linkedoptic
    (:`Is Valid`
      (`SKGProceduralAnimComponent.SetCanAim` (`SKGShooterFrameworkHelpers.GetProceduralAnimComponent` _linkedoptic) true)
      (`SKGFirearmComponent.SetAimingDevice` (`SKGShooterFrameworkHelpers.GetParentFirearmComponent` self) (`SKGShooterFrameworkHelpers.GetProceduralAnimComponent` (`self.LinkedOptic`)) (`self.GetIsAiming`))
      (`SKGProceduralAnimComponent.SetCanAim` (`self.SKGProceduralAnim_Magnifier`) false))))

(event `self.ReceiveDestroyed`
  (bind _linkedoptic (`self.LinkedOptic`))
  (bind _returnvalue (`SKGShooterFrameworkHelpers.GetProceduralAnimComponent` _linkedoptic))
  (if (`self.GetIsLocallyControlled`)
    (`/Engine/EditorBlueprintResources/StandardMacros.IsValid` _linkedoptic
      (:`Is Valid`
        (`SKGProceduralAnimComponent.SetCanAim` _returnvalue true)
        (`SKGFirearmComponent.SetAimingDevice` (`SKGShooterFrameworkHelpers.GetParentFirearmComponent` self) _returnvalue (`self.GetIsAiming`))))))

(event `FlipMagnifier`
  (if (`self.bCanBeFlipped`)
    (bind _output_get (set `self.bIsFlipped` (not (`self.bIsFlipped`))))
    (`/Engine/EditorBlueprintResources/ActorMacros.Switch Has Authority`
      (:`Authority`
        _)
      (:`Remote`
        (`self.Server_FlipMagnifier` _output_get)))
    (set `self.bCanBeFlipped` false)
    (`KismetSystemLibrary.Delay` (`self.DelayBetweenFlips`))
    (set `self.bCanBeFlipped` true)))

(event `Server_FlipMagnifier`
  (params (Flipped :type Boolean))
  (set `self.bIsFlipped` Flipped))

(event `self.Interact`
  (params (Pawn :type "Pawn Object Reference"))
  (bind _returnvalue (`SKGShooterFrameworkHelpers.GetParentWithFirearmComponent` self))
  (`/Engine/EditorBlueprintResources/StandardMacros.IsValid` _returnvalue
    (:`Is Valid`
      (bind _asinteract_interface (cast `InteractInterface` _returnvalue))
      (`InteractInterface.Interact` _asinteract_interface null))))

(event `self.SKGOptic.OnReticleCycled`
  (bind _returnvalue (`SKGShooterFrameworkHelpers.GetOpticComponent` (`self.LinkedOptic`)))
  (`/Engine/EditorBlueprintResources/StandardMacros.IsValid` _returnvalue
    (:`Is Valid`
      (`SKGOpticComponent.CycleReticle` _returnvalue))))

(event `self.SKGOptic.OnReticleBrightnessChanged`
  (params (bIncrease :type Boolean))
  (bind _returnvalue (`SKGShooterFrameworkHelpers.GetOpticComponent` (`self.LinkedOptic`)))
  (`/Engine/EditorBlueprintResources/StandardMacros.IsValid` _returnvalue
    (:`Is Valid`
      (if bIncrease
        (`SKGOpticComponent.IncreaseReticleBrightness` _returnvalue)
        (else
          (`SKGOpticComponent.DecreaseReticleBrightness` _returnvalue))))))

(event `self.SKGOptic.OnNightVisionModeChanged`
  (params (bNightVisionModeOn :type Boolean))
  (bind _returnvalue (`SKGShooterFrameworkHelpers.GetOpticComponent` (`self.LinkedOptic`)))
  (`/Engine/EditorBlueprintResources/StandardMacros.IsValid` _returnvalue
    (:`Is Valid`
      (`SKGOpticComponent.ToggleReticleNightVisionSetting` _returnvalue))))

(fn `Get Shooter Pawn Component`
  (returns (ReturnValue :type "SKGShooterPawnComponent Object Reference"))
  (bind _returnvalue (`SKGShooterFrameworkHelpers.GetParentWithFirearmComponent` self))
  (`/Engine/EditorBlueprintResources/StandardMacros.IsValid` _returnvalue
    (:`Is Valid`
      (return (`SKGShooterFrameworkHelpers.GetShooterPawnComponent` (`self.GetOwner` _returnvalue))))
    (:`Is Not Valid`
      (return null))))

(fn `GetIsAiming`
  (returns (ReturnValue :type Boolean))
  (bind _returnvalue (`self.Get Shooter Pawn Component`))
  (`/Engine/EditorBlueprintResources/StandardMacros.IsValid` _returnvalue
    (:`Is Valid`
      (return (`SKGShooterPawnComponent.bIsAiming` _returnvalue)))
    (:`Is Not Valid`
      (return false))))

(fn `GetIsLocallyControlled`
  (returns (ReturnValue :type Boolean))
  (bind _returnvalue (`self.Get Shooter Pawn Component`))
  (bind _returnvalue_2 (`SKGShooterPawnComponent.IsLocallyControlled` _returnvalue))
  (`/Engine/EditorBlueprintResources/StandardMacros.IsValid` _returnvalue
    (:`Is Valid`
      (if _returnvalue_2
        (return _returnvalue_2)
        (else
          _)))
    (:`Is Not Valid`
      _))
  (return false))

(fn `HandleFlippedResult`
  (locals (MeshToUse :type "SkeletalMeshComponent Object Reference"))
  (bind _skeletalmesh (`self.SkeletalMesh`))
  (bind _flippedpawnmontage (`self.FlippedPawnMontage`))
  (if (`self.bIsFlipped`)
    (`SkeletalMeshComponent.PlayAnimation` _skeletalmesh (`self.FlippedOutAnimation`) false)
    (`self.SetAimToLinkedOptic`)
    (`self.MagnifierFlipped` _flippedpawnmontage (`self.FlippedOutSectionName`))
    (else
      (`SkeletalMeshComponent.PlayAnimation` _skeletalmesh (`self.FlippedInAnimation`) false)
      (if (or (`self.GetIsLocallyControlled`) (`self.HasAuthority`))
        (`self.SetAimToMagnifier`)
        (`self.MagnifierFlipped` _flippedpawnmontage (`self.FlippedInSectionName`))))))

(fn `LinkOptic`
  (locals (OpticActors :type "Array of Actor Object Reference") (ClosestActor :type "Actor Object Reference") (ClosestDistance :type "Float (double-precision)" :default 10000000.0))
  (bind _returnvalue (`self.K2_GetActorLocation`))
  (bind _outhits (`KismetSystemLibrary.SphereTraceMulti` _returnvalue (+ _returnvalue (* (`self.GetActorRightVector`) 15.0)) 1.75 "TraceTypeQuery1"))
  (for _array_element _outhits
    (bind (_bblockinghit _binitialoverlap _time _distance _location _impactpoint _normal _impactnormal _physmat _hitactor) (`GameplayStatics.BreakHitResult` _array_element))
    (`/Engine/EditorBlueprintResources/StandardMacros.IsValid` (`SKGShooterFrameworkHelpers.GetOpticComponent` _hitactor)
      (:`Is Valid`
        (`KismetArrayLibrary.Array_Add` (`local.OpticActors`) _hitactor))))
  (for _array_element_2 (`local.OpticActors`)
    (bind _returnvalue_2 (`KismetMathLibrary.Vector_Distance` (`self.K2_GetActorLocation` _array_element_2) (`self.K2_GetActorLocation`)))
    (if (< _returnvalue_2 (`local.ClosestDistance`))
      (set `local.ClosestDistance` _returnvalue_2)
      (set `local.ClosestActor` _array_element_2)))
  (set `self.LinkedOptic` (`local.ClosestActor`))
  (`self.HandleFlippedResult`))

(fn `OnRep_bIsFlipped`
  (`self.HandleFlippedResult`))

(fn `OnRep_LinkedOptic`)

(fn `UserConstructionScript`)