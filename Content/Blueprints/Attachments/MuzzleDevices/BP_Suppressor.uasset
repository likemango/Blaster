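; Suppressor muzzle attachment that visually shows barrel heat through the SKG muzzle temperature system.
; On BeginPlay, if that system is in use, it creates a dynamic material on the static mesh.
; Temperature changes feed the normalized value into the material and the Niagara heat smoke, which runs only while the value is above zero.
; Interact calls are forwarded to the parent that has a firearm component.
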(event `self.ReceiveBeginPlay`
  (bind _staticmesh (`self.StaticMesh`))
  (if (`SKGMuzzleComponent.IsUsingMuzzleTemperatureSystem` (`self.SKGMuzzle_Suppressor`))
    (bind _returnvalue (`PrimitiveComponent.CreateDynamicMaterialInstance` _staticmesh 0 (`PrimitiveComponent.GetMaterial` _staticmesh 0) "None"))
    (bind _output_get (set `self.MuzzleMaterial` _returnvalue))
    (`PrimitiveComponent.SetMaterial` (`self.StaticMesh`) 0 _output_get)))

(event `self.SKGMuzzle_Suppressor.OnMuzzleTemperatureChanged`
  (params (Temperature :type "Float (single-precision)"))
  (bind _ns_heatsmoke (`self.NS_HeatSmoke`))
  (bind _returnvalue (`SKGMuzzleComponent.GetMuzzleTemperatureNormalized` (`self.SKGMuzzle_Suppressor`)))
  (`MaterialInstanceDynamic.SetScalarParameterValue` (`self.MuzzleMaterial`) "NormalizedTemperature" _returnvalue)
  (if (> _returnvalue 0.0)
    (if (not (`ActorComponent.IsActive` _ns_heatsmoke))
      (`ActorComponent.Activate` _ns_heatsmoke false))
    (`NiagaraComponent.SetVariableFloat` (`self.NS_HeatSmoke`) "MuzzleTemp" _returnvalue)
    (else
      (`ActorComponent.Deactivate` _ns_heatsmoke))))

(event `self.Interact`
  (params (Pawn :type "Pawn Object Reference"))
  (bind _returnvalue (`SKGShooterFrameworkHelpers.GetParentWithFirearmComponent` self))
  (`/Engine/EditorBlueprintResources/StandardMacros.IsValid` _returnvalue
    (:`Is Valid`
      (message `/Game/Blueprints/Attachments/MuzzleDevices/BP_Suppressor.Interact` _returnvalue Pawn))))

(fn `UserConstructionScript`)