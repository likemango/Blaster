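; BP_LPVONoSceneCapture is an LPVO scope attachment that, by its name, works without scene capture.
; On BeginPlay it hands its mesh and the MPC_ScopeMask material parameter collection to the SKG optic subsystem through SetTickTest.
; Interact calls are forwarded to the parent that has a firearm component.
; A disconnected node that writes the S_Aim socket location to the collection's ScopeLocation parameter never runs.
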(event `self.ReceiveBeginPlay`
  (`SKGOpticSubsystem.SetTickTest` (subsystem `SKGOpticSubsystem`) (`self.StaticMesh`) "/Game/Blueprints/Attachments/Optics/NewFolder/MPC_ScopeMask.MPC_ScopeMask"))

(event `self.ReceiveTick`
  (params (DeltaSeconds :type "Float (single-precision)")))

(event `self.Interact`
  (params (Pawn :type "Pawn Object Reference"))
  (bind _returnvalue (`SKGShooterFrameworkHelpers.GetParentWithFirearmComponent` self))
  (`/Engine/EditorBlueprintResources/StandardMacros.IsValid` _returnvalue
    (:`Is Valid`
      (message `/Game/Blueprints/Attachments/Optics/NewFolder/BP_LPVONoSceneCapture.Interact` _returnvalue Pawn))))

(fn `UserConstructionScript`)