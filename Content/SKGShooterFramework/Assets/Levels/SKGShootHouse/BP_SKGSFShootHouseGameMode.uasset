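; Game mode for the SKG shoot house level that spawns AI enemies and tracks their live count.
; On BeginPlay it sorts spawn point actors into initial and respawn lists, then spawns the starting AI at random initial points.
; Killed AI decrement the count and despawn after a random delay, while MaintainAICount spawns one at a respawn point when below target.
; ReloadLevel restarts the map as a listen server through ServerTravel.
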(event `self.ReceiveBeginPlay`
  (`self.SetupAISpawnPoints`)
  (`self.SpawnInitialAI`))

(event `ReloadLevel`
  (`KismetSystemLibrary.ExecuteConsoleCommand` (`KismetStringLibrary.Concat_StrStr` "ServerTravel " (`self.LevelName`) "?listen") null))

(event `SetupAISpawnPoints`
  (bind _outactors (`GameplayStatics.GetAllActorsOfClass` "/Game/SKGShooterFramework/Blueprints/Pawn/AI/BP_SKGSFAISpawnPoint.BP_SKGSFAISpawnPoint_C"))
  (bind _output_get (set `self.AISpawnPoints` _outactors))
  (for _array_element _output_get
    (if (`/Game/SKGShooterFramework/Blueprints/Pawn/AI/BP_SKGSFAISpawnPoint.bIsRespawnPoint` _array_element)
      (`KismetArrayLibrary.Array_Add` (`self.AIRespawnPoints`) _array_element)
      (else
        (`KismetArrayLibrary.Array_Add` (`self.AIInitialSpawnPoints`) _array_element)))))

(event `SpawnInitialAI`
  (for _ (range 1 (+ (`self.InitialAISpawnCount`) 1))
    (`self.SpawnAIAtRandomPoint` (`self.AIInitialSpawnPoints`))))

(event `SpawnAIAtRandomPoint`
  (params (SpawnPoints :type "Array of /Game/SKGShooterFramework/Blueprints/Pawn/AI/BP_SKGSFAISpawnPoint Object Reference"))
  (`|SpawnActorFromClass` (`self.AISpawnClass`) (`self.GetTransform` (`KismetArrayLibrary.Array_Random` SpawnPoints)) "AdjustIfPossibleButAlwaysSpawn" "MultiplyWithRoot" null null)
  (`self.AddAICount`))

(event `AddAICount`
  (bind _result (`/Engine/EditorBlueprintResources/StandardMacros.IncrementInt` (`self.CurrentAICount`))
    (:`  `
      (set `self.CurrentAICount` _result))))

(event `RemoveAICount`
  (bind _result (`/Engine/EditorBlueprintResources/StandardMacros.DecrementInt` (`self.CurrentAICount`))
    (:`  `
      (set `self.CurrentAICount` _result))))

(event `OnAIKilled`
  (params (Pawn :type "Pawn Object Reference"))
  (`self.RemoveAICount`)
  (`self.SetLifeSpan` Pawn (`KismetMathLibrary.RandomFloatInRange` (`self.AIKilledCleanupMinTime`) (`self.AIKilledCleanupMaxTime`))))

(event `MaintainAICount`
  (if (< (`self.CurrentAICount`) (`self.AIMaintainCount`))
    (`self.SpawnAIAtRandomPoint` (`self.AIRespawnPoints`))))

(fn `UserConstructionScript`)