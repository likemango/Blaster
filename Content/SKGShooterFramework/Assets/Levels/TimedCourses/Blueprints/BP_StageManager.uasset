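; Stage manager for a timed shooting course that times a run from start to stop and adds target penalties.
; On authority it binds to the start and stop objects, recording the starting pawn and computing total time.
; RepNotify on active state and total time fires dispatchers for the bound time display, and resets targets when the stage deactivates.
; Targets receive the manager through messages, and the construction script labels the stage.
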(event `self.ReceiveBeginPlay`
  (`self.SetupStageTargets`)
  (`/Game/SKGShooterFramework/Assets/Levels/TimedCourses/Blueprints/BP_StageTimeDisplay.BindToStageManager` (`self.StageTimeDisplay`) self)
  (`/Engine/EditorBlueprintResources/ActorMacros.Switch Has Authority`
    (:`Authority`
      (`self.BindToStageStartStop`))))

(event `BindToStageStartStop`
  (add `/Game/SKGShooterFramework/Assets/Levels/TimedCourses/Blueprints/BP_StageStartStopPoint.StageStarted` (`self.StageStart`) (`|CreateDelegate` :!event `StageStarted`))
  (add `/Game/SKGShooterFramework/Assets/Levels/TimedCourses/Blueprints/BP_StageStartStopPoint.StageStopped` (`self.StageStop`) (`|CreateDelegate` :!event `StageStopped`)))

(event `StageStarted`
  (params (Pawn :type "Pawn Object Reference"))
  (set `self.bStageActive` true)
  (set `self.StageStartOwner` Pawn)
  (set `self.StageStartTime` (`GameplayStatics.GetTimeSeconds`))
  (set `self.StageTotalTime` 0.0))

(event `StageStopped`
  (if (`self.bStageActive`)
    (`self.SetTotalStageTime`)
    (set `self.bStageActive` false)))

(event `SetTotalStageTime`
  (`self.AddUpPenalties`)
  (set `self.StageTotalTime` (+ (`self.Penalties`) (- (`GameplayStatics.GetTimeSeconds`) (`self.StageStartTime`)))))

(event `SetupStageTargets`
  (for _array_element (`self.Targets`)
    (message `/Game/SKGShooterFramework/Assets/Levels/TimedCourses/Blueprints/Interfaces/BPI_StageTarget.SetStageManager` _array_element self)))

(event `ResetTargets`
  (for _array_element (`self.Targets`)
    (message `/Game/SKGShooterFramework/Assets/Levels/TimedCourses/Blueprints/Interfaces/BPI_StageTarget.ResetTarget` _array_element)))

(event `AddUpPenalties`
  (set `self.Penalties` 0.0)
  (for _array_element (`self.Targets`)
    (bind _penalty (message `/Game/SKGShooterFramework/Assets/Levels/TimedCourses/Blueprints/Interfaces/BPI_StageTarget.GetPenalty` _array_element))
    (set `self.Penalties` (+ _penalty (`self.Penalties`)))))

(fn `OnRep_bStageActive`
  (if (`self.bStageActive`)
    (`self.StageActive`)
    (else
      (`self.ResetTargets`)
      (`self.StageDeactive`))))

(fn `OnRep_StageTotalTime`
  (`self.StageFinalTimeSet` (`self.StageTotalTime`)))

(fn `UserConstructionScript`
  (`TextRenderComponent.K2_SetText` (`self.TextRender`) (`KismetTextLibrary.Conv_StringToText` (`self.StageName`))))