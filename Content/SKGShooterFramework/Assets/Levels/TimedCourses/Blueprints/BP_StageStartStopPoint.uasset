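; Trigger point that marks either the start or the completion of a timed course stage, selected by the IsStopPoint flag.
; When a pawn overlaps the box on the server, it calls the stage started dispatcher with that pawn and plays a start sound, or calls the stage stopped dispatcher.
; The construction script sets the label to green "Start Stage" or red "Complete Stage" to match the flag.
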(event `self.Box.OnComponentBeginOverlap`
  (params (OverlappedComponent :type "PrimitiveComponent Object Reference") (OtherActor :type "Actor Object Reference") (OtherComp :type "PrimitiveComponent Object Reference") (OtherBodyIndex :type Integer) (bFromSweep :type Boolean) (SweepResult :type "HitResult Structure (by ref)"))
  (`/Engine/EditorBlueprintResources/ActorMacros.Switch Has Authority`
    (:`Authority`
      (bind _aspawn (cast `Pawn` OtherActor))
      (if (`self.bIsStopPoint`)
        (`self.StageStopped`)
        (else
          (`self.StageStarted` _aspawn)
          (`GameplayStatics.PlaySoundAtLocation` (`self.StartSound`) (`self.K2_GetActorLocation`) (struct) 1.0 1.0 0.0 null null null null))))))

(fn `UserConstructionScript`
  (bind _textrender (`self.TextRender`))
  (if (`self.bIsStopPoint`)
    (`TextRenderComponent.K2_SetText` _textrender "Complete Stage")
    (`TextRenderComponent.SetTextRenderColor` (`self.TextRender`) (make `Color` 0 0 255 255))
    (else
      (`TextRenderComponent.K2_SetText` _textrender "Start Stage")
      (`TextRenderComponent.SetTextRenderColor` (`self.TextRender`) (make `Color` 0 255 0 255)))))