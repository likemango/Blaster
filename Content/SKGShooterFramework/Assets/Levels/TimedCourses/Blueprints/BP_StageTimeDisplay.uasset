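; BP_StageTimeDisplay is a text display actor that shows the elapsed time for a stage in a timed course.
; It binds to a stage manager's active, deactive and final-time-set events.
; Activation records the start time and enables tick, which refreshes the TextRender with time elapsed since then.
; Deactivation disables tick, and the final-time event writes the time supplied by the manager.
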(event `BindToStageManager`
  (params (Manager :type "/Game/SKGShooterFramework/Assets/Levels/TimedCourses/Blueprints/BP_StageManager Object Reference"))
  (bind _output_get (set `self.StageManager` Manager))
  (add `/Game/SKGShooterFramework/Assets/Levels/TimedCourses/Blueprints/BP_StageManager.StageActive` _output_get (`|CreateDelegate` :!event `StageActivated`))
  (add `/Game/SKGShooterFramework/Assets/Levels/TimedCourses/Blueprints/BP_StageManager.StageDeactive` _output_get (`|CreateDelegate` :!event `StageDeactivated`))
  (add `/Game/SKGShooterFramework/Assets/Levels/TimedCourses/Blueprints/BP_StageManager.StageFinalTimeSet` _output_get (`|CreateDelegate` :!event `SetFinalTime`)))

(event `self.ReceiveTick`
  (params (DeltaSeconds :type "Float (single-precision)"))
  (`TextRenderComponent.K2_SetText` (`self.TextRender`) (`self.GetTimeText`)))

(event `StageActivated`
  (set `self.StartCountTime` (`GameplayStatics.GetTimeSeconds`))
  (`self.SetActorTickEnabled` true))

(event `StageDeactivated`
  (`self.SetActorTickEnabled` false))

(event `SetFinalTime`
  (params (Time :type "Float (double-precision)"))
  (`TextRenderComponent.K2_SetText` (`self.TextRender`) (`KismetTextLibrary.Conv_DoubleToText` Time "HalfToEven")))

(fn `GetTimeText`
  (returns (Time :type Text))
  (return (`KismetTextLibrary.Conv_DoubleToText` (- (`GameplayStatics.GetTimeSeconds`) (`self.StartCountTime`)) "HalfToEven")))

(fn `UserConstructionScript`)