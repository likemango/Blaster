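; BP_IPSC is an IPSC target for timed courses that reports a failure-to-neutralize penalty to scoring.
; It stores a stage manager reference, and resetting the target clears its hit count.
; GetPenalty returns zero once hits reach the required count, otherwise the penalty value.
; The Hit event is empty, and the hit-counting logic gated on an active stage is unconnected, so this graph never increments hits.
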(event `/Game/SKGShooterFramework/Blueprints/Interfaces/BPI_Hit.Hit`
  (params (DamageAmount :type "Float (double-precision)") (HitResult :type "HitResult Structure")))

(event `/Game/SKGShooterFramework/Assets/Levels/TimedCourses/Blueprints/Interfaces/BPI_StageTarget.SetStageManager`
  (params (Manager :type "/Game/SKGShooterFramework/Assets/Levels/TimedCourses/Blueprints/BP_StageManager Object Reference"))
  (set `self.StageManager` Manager))

(event `/Game/SKGShooterFramework/Assets/Levels/TimedCourses/Blueprints/Interfaces/BPI_StageTarget.ResetTarget`
  (set `self.CurrentHits` 0))

(fn `GetPenalty`
  (returns (Penalty :type "Float (double-precision)"))
  (if (>= (`self.CurrentHits`) (`self.HitsRequired`))
    (return 0.0)
    (else
      (return (`self.FailureToNeutralizePenalty`)))))

(fn `UserConstructionScript`)