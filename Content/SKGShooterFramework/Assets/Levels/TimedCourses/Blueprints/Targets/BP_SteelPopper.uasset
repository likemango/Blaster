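; Steel popper target for timed shooting courses that falls when hit and reports a failure-to-neutralize penalty while it is not hit.
; A hit sets a flag and plays the down animation, then after a short delay the target resets itself and plays the up animation.
; The stage manager reference is stored, but the stage-active check that uses it is disconnected, so hits register regardless of stage state.
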(event `self.Hit`
  (params (DamageAmount :type "Float (double-precision)") (HitResult :type "HitResult Structure"))
  (if (not (`self.bHit`))
    (set `self.bHit` true)
    (`self.TargetDown`)
    (`KismetSystemLibrary.Delay` 2.0)
    (`self.ResetTarget`)))

(event `self.SetStageManager`
  (params (Manager :type "/Game/SKGShooterFramework/Assets/Levels/TimedCourses/Blueprints/BP_StageManager Object Reference"))
  (set `self.StageManager` Manager))

(event `self.ResetTarget`
  (set `self.bHit` false)
  (`self.TargetUp`))

(event `TargetDown`
  (`SkeletalMeshComponent.PlayAnimation` (`self.SkeletalMesh`) "/Game/SKGShooterFramework/Assets/Targets/Steel/SteelPopper/A_SteelPopper_Down.A_SteelPopper_Down" false))

(event `TargetUp`
  (`SkeletalMeshComponent.PlayAnimation` (`self.SkeletalMesh`) "/Game/SKGShooterFramework/Assets/Targets/Steel/SteelPopper/A_SteelPopper_Up.A_SteelPopper_Up" false))

(fn `GetPenalty`
  (returns (Penalty :type "Float (double-precision)"))
  (if (`self.bHit`)
    (return 0.0)
    (else
      (return (`self.FailureToNeutralizePenalty`)))))

(fn `UserConstructionScript`)